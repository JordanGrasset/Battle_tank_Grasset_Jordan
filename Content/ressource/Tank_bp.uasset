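; Tank Blueprint that handles player aiming of the camera rig, turret and barrel; it contains no driving or firing logic.
; The AimAzimuth axis yaws both the AzimutGameMode component and the Turret, while AimAltitude pitches both the SpringArm and the Barrel.
; Each rotation is local, scaled by world delta seconds and a fixed rate, with no explicit pitch clamp.
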(event Input|AxisEvents|InputAxisAimAzimuth
  (params (AxisValue :type Float%20%28single-precision%29))
  ;[1 1 1] Deplacement Horizontal
  (Transformation|AddLocalRotation (Variables|Default|GetAzimutGameMode) (Math|Rotator|MakeRotator 0.0 0.0 (* AxisValue (Utilities|Time|GetWorldDeltaSeconds) 1e+02)) false false))

(event Input|AxisEvents|InputAxisAimAzimuth
  (params (AxisValue :type Float%20%28single-precision%29))
  ;[1 1 1] Rotation Turret
  (Transformation|AddLocalRotation (Variables|Default|GetTurret) (Math|Rotator|MakeRotator 0.0 0.0 (* AxisValue (Utilities|Time|GetWorldDeltaSeconds) 1e+02)) false false))

(event Input|AxisEvents|InputAxisAimAltitude
  (params (AxisValue :type Float%20%28single-precision%29))
  ;[1 1 1] Deplacement Vertical
  (Transformation|AddLocalRotation (Variables|Default|GetSpringArm) (Math|Rotator|MakeRotator 0.0 (* AxisValue (Utilities|Time|GetWorldDeltaSeconds) 1e+02) 0.0) false false))

(event Input|AxisEvents|InputAxisAimAltitude
  (params (AxisValue :type Float%20%28single-precision%29))
  ;[1 1 1] Translation Barrel
  (Transformation|AddLocalRotation (Variables|Default|GetBarrel) (Math|Rotator|MakeRotator 0.0 (* AxisValue (Utilities|Time|GetWorldDeltaSeconds) 1e+02) 0.0) false false))

(fn ConstructionScript)